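; Interactable terminal that drops the shield of its linked BP_Core for a limited time, with an overlap sphere showing the interaction prompt.
; Deactivation recolors the sprite, fades the force field via timeline, disables its collision and enables core damage.
; A Tick countdown then triggers reactivation, reversing these changes and re-arming the terminal.
; Tick also toggles the core health widget, and shield changes are broadcast through the SPM game instance subsystem.
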(event `OnCoreDeactivated_Event`
  (bind _core (`self.Core`))
  (bind _spherecomponent (`self.SphereComponent`))
  ;[1 1 1] När coren ska bli deactiverad så körs detta
  (`|ExecutionSequence`
    (:`then_0`
      (set `self.IsShieldDown` true))
    (:`then_1`
      (`PaperSpriteComponent.SetSpriteColor` (`self.PaperSprite`) (struct :`R` 0.049486 :`G` 1.0 :`A` 1.0))
      (`|ExecutionSequence`
        (:`then_0`
          (remove `PrimitiveComponent.OnComponentBeginOverlap` _spherecomponent (delegate `OnComponentBeginOverlap`)))
        (:`then_1`
          (remove `PrimitiveComponent.OnComponentEndOverlap` _spherecomponent (delegate `OnComponentEndOvelap`))
          (`Widget.RemoveFromParent` (stale `self.ReceiveBeginPlay` _output_get) :!label _label))
        (:`then_2`
          (`/Engine/EditorBlueprintResources/StandardMacros.IsValid` _core
            (:`Is Valid`
              (bind _asbp_core (cast `/Game/CoreSysten/BP_Core` _core)
                (:`then`
                  (bind (_direction _alpha) (`Timeline|Timeline`)
                    (:`Update`
                      (bind _forcefield (`/Game/CoreSysten/BP_Core.ForceField` _asbp_core))
                      (`/Engine/EditorBlueprintResources/StandardMacros.IsValid` _forcefield
                        (:`Is Valid`
                          (`MeshComponent.SetScalarParameterValueOnMaterials` _forcefield "Alpha" _alpha)
                          (`PrimitiveComponent.SetCollisionEnabled` (`/Game/CoreSysten/BP_Core.ForceFieldCollision` _asbp_core) "NoCollision")
                          (bind _returnvalue (`self.Should Show Core Health` _asbp_core))
                          (set `self.ShowCoreHealth` _returnvalue)
                          (`GameplayStatics.PlaySound2D` "/Game/Audio/SFX/Objectives/Core/SFX_Objective_Core_Shield_Deactivate.SFX_Objective_Core_Shield_Deactivate" 1.0 1.0 0.0 null null)
                          (`AudioComponent.Stop` (`/Game/CoreSysten/BP_Core.Audio` _asbp_core))
                          (`SPMGameInstanceSubsystem.OnCoreDeactivated` (subsystem `SPMGameInstanceSubsystem`) (`self.Core`)))))))
                (:`CastFailed`
                  (`KismetSystemLibrary.PrintString` "Cast Faild"))))))
        (:`then_3`
          (`HealthComponent.ActivateTakeDamage` (`BaseCore.HealthComponent` _asbp_core)))))))

(event `self.ReceiveBeginPlay`
  (bind _spherecomponent (`self.SphereComponent`))
  ;[1 1 1] Begin Play sets events and diffretn Variables
  (bind _returnvalue (`|CreateWidget` "/Game/Interactions/WB_InteractionPrompt.WB_InteractionPrompt_C"))
  (bind _output_get (set `self.UserWidget` _returnvalue))
  (add `self.OnCoreDisabled` (delegate `OnCoreDeactivated_Event`))
  (add `self.OnCoreReActive` (delegate `OnCoreReactivated`))
  (add `PrimitiveComponent.OnComponentBeginOverlap` _spherecomponent (delegate `OnComponentBeginOverlap`))
  (add `PrimitiveComponent.OnComponentEndOverlap` _spherecomponent (delegate `OnComponentEndOvelap`))
  (set `self.Timer` (`self.DefaultTimer`))
  (add `SPMGameInstanceSubsystem.OnCoreDestroyed` (subsystem `SPMGameInstanceSubsystem`) (delegate `CoreDestroyed`)))

(event `OnComponentEndOvelap`
  (params (OverlappedComponent :type "PrimitiveComponent Object Reference") (OtherActor :type "Actor Object Reference") (OtherComp :type "PrimitiveComponent Object Reference") (OtherBodyIndex :type Integer))
  (goto _label))

(event `OnComponentBeginOverlap`
  (params (OverlappedComponent :type "PrimitiveComponent Object Reference") (OtherActor :type "Actor Object Reference") (OtherComp :type "PrimitiveComponent Object Reference") (OtherBodyIndex :type Integer) (bFromSweep :type Boolean) (SweepResult :type "HitResult Structure (by ref)"))
  (`UserWidget.AddToViewport` (stale `self.ReceiveBeginPlay` _output_get) 0))

(event `CoreDestroyed`
  (params (Core :type "BaseCore Object Reference"))
  (bind _core (`self.Core`))
  (clear `self.OnCoreReActive`)
  (`/Engine/EditorBlueprintResources/StandardMacros.IsValid` _core
    (:`Is Valid`
      (set `self.IsCoreDead` (<= (`HealthComponent.GetHealthPercentage` (`self.GetComponentByClass` _core "/Script/SPM.HealthComponent")) 0.0)))
    (:`Is Not Valid`
      (set `self.IsCoreDead` true))))

(event `self.ReceiveTick`
  (params (DeltaSeconds :type "Float (single-precision)"))
  ;[1 1 1] Tick för att utföra en timer när corens sköld ska aktiveras
  (`|ExecutionSequence`
    (:`then_0`
      (if (`self.IsShieldDown`)
        (bind _output_get (set `self.Timer` (- (`self.Timer`) DeltaSeconds)))
        (if (<= _output_get 0.0)
          (`self.OnCoreReActive`)
          (set `self.Timer` (`self.DefaultTimer`)))))
    (:`then_1`
      (if (not (`self.IsCoreDead`))
        (bind _asbp_core (cast `/Game/CoreSysten/BP_Core` (`self.Core`)))
        (bind _returnvalue (`self.Should Show Core Health` _asbp_core))
        (if (and (`self.ShowCoreHealth`) _returnvalue)
          (bind _corehealthwidget (`/Game/CoreSysten/BP_Core.CoreHealthWidget` _asbp_core))
          (`Widget.SetVisibility` _corehealthwidget "Visible")
          (else
            (`Widget.SetVisibility` _corehealthwidget "Hidden")))))))

(event `OnCoreReactivated`
  (bind _spherecomponent (`self.SphereComponent`))
  ;[1 1 1] När coren ska activeras igen så ändra de nödvändiga sakerna
  (`|ExecutionSequence`
    (:`then_0`
      (set `self.IsShieldDown` false))
    (:`then_1`
      (`PaperSpriteComponent.SetSpriteColor` (`self.PaperSprite`) (struct :`R` 1.0 :`B` 0.143847 :`A` 1.0))
      (`|ExecutionSequence`
        (:`then_0`
          (add `PrimitiveComponent.OnComponentBeginOverlap` _spherecomponent (delegate `OnComponentBeginOverlap`)))
        (:`then_1`
          (add `PrimitiveComponent.OnComponentEndOverlap` _spherecomponent (delegate `OnComponentEndOvelap`)))
        (:`then_2`
          (bind _asbp_core (cast `/Game/CoreSysten/BP_Core` (`self.Core`)))
          (`|ExecutionSequence`
            (:`then_0`
              (bind _forcefield (`/Game/CoreSysten/BP_Core.ForceField` _asbp_core))
              (`SceneComponent.SetVisibility` _forcefield true true)
              (`PrimitiveComponent.SetCollisionEnabled` (`/Game/CoreSysten/BP_Core.ForceFieldCollision` _asbp_core) "QueryAndPhysics")
              (bind _returnvalue (`self.Should Show Core Health` _asbp_core))
              (set `self.ShowCoreHealth` _returnvalue)
              (`AudioComponent.Play` (`/Game/CoreSysten/BP_Core.Audio` _asbp_core) 0.0)
              (`KismetSystemLibrary.PrintText` "Hello")
              (`SPMGameInstanceSubsystem.OnCoreActivated` (subsystem `SPMGameInstanceSubsystem`) (`self.Core`)))
            (:`then_1`
              (bind (_direction _alpha) (`Timeline|Timeline_0` :!via `Reverse`)
                (:`Update`
                  (`MeshComponent.SetScalarParameterValueOnMaterials` _forcefield "Alpha" _alpha)
                  (`HealthComponent.DisableTakeDamage` (`BaseCore.HealthComponent` _asbp_core)))))))
        (:`then_3`
          (`self.SetInteractableOnDisable`)
          (`GameplayStatics.PlaySound2D` "/Game/Audio/SFX/Objectives/Core/SFX_Objective_Core_Shield_Activate.SFX_Objective_Core_Shield_Activate" 1.0 1.0 0.0 null null))))))

(fn `Should Show Core Health`
  (params (Core :type "/Game/CoreSysten/BP_Core Object Reference"))
  (returns (ReturnValue :type Boolean))
  (return (and (`PrimitiveComponent.IsOverlappingActor` (`/Game/CoreSysten/BP_Core.CoreHealthCollider` Core) (`GameplayStatics.GetPlayerCharacter` 0)) (> (`HealthComponent.GetHealth` (`self.GetComponentByClass` Core "/Script/SPM.HealthComponent")) 0.0))))

(fn `UserConstructionScript`)