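; BP_Core is a destructible core objective with a hidden health widget and damage disabled at BeginPlay.
; Tick spawns sparks once when health drops below a threshold.
; On death it explodes with camera shake, teleports to a fixed location, lowers the MasterMind token limit and fades in the player's next objective.
; It also sends checkpoint messages to the game mode for itself, player health and transform, and the electricity door.
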(event `self.ReceiveBeginPlay`
  (bind _returnvalue (`|CreateWidget` "/Game/UI/WB_CoreHealth.WB_CoreHealth_C" (`GameplayStatics.GetPlayerController` 0)))
  (bind _output_get (set `self.CoreHealthWidget` _returnvalue))
  (`UserWidget.AddToViewport` _output_get 0)
  (`Widget.SetVisibility` _output_get "Hidden")
  (`HealthComponent.DisableTakeDamage` (`self.HealthComponent`)))

(event `self.ReceiveDestroyed`
  (`|ExecutionSequence`
    (:`then_0`
      (`Widget.RemoveFromParent` (`self.CoreHealthWidget`))
      (set `self.CoreHealthWidget` null))
    (:`then_1`
      (`NiagaraFunctionLibrary.SpawnSystemAtLocation` "/Game/Particle/Explosion/Explosion.Explosion" (`self.K2_GetActorLocation` self) (`self.K2_GetActorRotation` self))
      (`LegacyCameraShake.StartLegacyCameraShake` null "/Script/GameplayCameras.LegacyCameraShake" 10.0))
    (:`then_2`
      (message `/Game/SaveSystem/BPI_SaveObjects.SaveDestroyedObject` (`GameplayStatics.GetGameMode`) self))))

(event `self.ReceiveTick`
  (params (DeltaSeconds :type "Float (single-precision)"))
  ;[1 1 1] Ligger på IS
  (`|ExecutionSequence`
    (:`then_1`
      (if (and (`self.CanPlay`) (< (`HealthComponent.GetHealthPercentage` (`self.GetComponentByClass` self "/Script/SPM.HealthComponent")) (`self.Percentage`)))
        (`NiagaraFunctionLibrary.SpawnSystemAttached` "/Game/Particle/NG_Sparks1.NG_Sparks1" null "None" (`self.K2_GetActorLocation` self) (`self.K2_GetActorRotation` self) "KeepWorldPosition")
        (set `self.CanPlay` false)))))

(event `self.HealthComponent.OnDead`
  (`self.DestroyCore`)
  (`|ExecutionSequence`
    (:`then_0`
      (`Widget.RemoveFromParent` (`self.CoreHealthWidget`))
      (set `self.CoreHealthWidget` null))
    (:`then_1`
      (`NiagaraFunctionLibrary.SpawnSystemAtLocation` "/Game/Particle/Explosion/Explosion.Explosion" (`self.K2_GetActorLocation` self) (`self.K2_GetActorRotation` self))
      (`GameplayStatics.PlayWorldCameraShake` "/Game/CoreSysten/CoreCameraShake.CoreCameraShake_C" (`self.K2_GetActorLocation`) 0.0 2000.0 1.0 true)
      (`self.K2_SetActorLocation` (7225.0 -15010.0 -1225.0) false true))
    (:`then_2`
      (`self.SaveGameState`))
    (:`then_3`
      (`MasterMindInstancedSubsystem.ReduceTokenLimit` (subsystem `MasterMindInstancedSubsystem`) 1.0))
    (:`then_4`
      (bind _asbp_first_person_character (cast `/Game/FirstPerson/Blueprints/BP_FirstPersonCharacter` (`GameplayStatics.GetPlayerCharacter` 0)))
      (bind _stepbystepobjective (`/Game/FirstPerson/Blueprints/BP_FirstPersonCharacter.StepByStepObjective` _asbp_first_person_character))
      (bind _fadeout (`/Game/UI/Objectives/StepByStepMissions/WB_StepByStepObjective.FadeOut` _stepbystepobjective))
      (if (not (`UserWidget.IsAnimationPlaying` _stepbystepobjective _fadeout))
        (`UserWidget.PlayAnimation` _stepbystepobjective _fadeout 0.0 1 "Forward" 1.0 false)
        (`KismetSystemLibrary.Delay` 0.5)
        (`/Game/FirstPerson/Blueprints/BP_FirstPersonCharacter.UpdateObjective` _asbp_first_person_character (`self.New Objective`) (`self.Details`))
        (bind _fadein (`/Game/UI/Objectives/StepByStepMissions/WB_StepByStepObjective.FadeIn` _stepbystepobjective))
        (if (not (`UserWidget.IsAnimationPlaying` _stepbystepobjective _fadein))
          (`UserWidget.PlayAnimation` _stepbystepobjective _fadein 0.0 1 "Forward" 1.0 false)
          (`KismetSystemLibrary.Delay` 1.2))))))

(fn `SaveGameState`
  (bind _returnvalue (`GameplayStatics.GetGameMode`))
  (bind _returnvalue_2 (`GameplayStatics.GetPlayerCharacter` 0))
  (bind _electricitydoor (`self.ElectricityDoor`))
  ;[1 1 1] Save game (checkpoint) after every destroyed core
  (message `/Game/SaveSystem/BPI_SaveObjects.SaveDestroyedObject` _returnvalue self)
  (message `/Game/SaveSystem/BPI_SaveObjects.SavePlayerHealth` _returnvalue)
  (message `/Game/SaveSystem/BPI_SaveObjects.SavePlayerPosition` _returnvalue (`self.K2_GetActorLocation` _returnvalue_2) (`self.K2_GetActorRotation` _returnvalue_2))
  (`/Engine/EditorBlueprintResources/StandardMacros.IsValid` _electricitydoor
    (:`Is Valid`
      (message `/Game/SaveSystem/BPI_SaveObjects.SaveLevelStream` (`GameplayStatics.GetGameMode`) _electricitydoor))
    (:`Is Not Valid`)))

(fn `UserConstructionScript`)