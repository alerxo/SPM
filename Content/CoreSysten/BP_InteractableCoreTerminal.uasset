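; Core terminal actor that shows a "Cores To Destoy" objective counter and an interaction prompt.
; BeginPlay creates both widgets, displays the objective and binds to the game instance subsystem's core-destroyed event.
; That event plays a sound and sets the count to Cores length minus one, without modifying the array.
; Sphere overlap shows the prompt when active; end overlap only refreshes objective text, leaving prompt removal unconnected.
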(event `self.SphereComponent.OnComponentBeginOverlap`
  (params (OverlappedComponent :type "PrimitiveComponent Object Reference") (OtherActor :type "Actor Object Reference") (OtherComp :type "PrimitiveComponent Object Reference") (OtherBodyIndex :type Integer) (bFromSweep :type Boolean) (SweepResult :type "HitResult Structure (by ref)"))
  (if (`self.bIsActive`)
    (`UserWidget.AddToViewport` (stale `self.ReceiveBeginPlay` _output_get_3) 0)))

(event `self.SphereComponent.OnComponentEndOverlap`
  (params (OverlappedComponent :type "PrimitiveComponent Object Reference") (OtherActor :type "Actor Object Reference") (OtherComp :type "PrimitiveComponent Object Reference") (OtherBodyIndex :type Integer))
  (`EditableText.SetText` (`/Game/Interactions/WB_ObjectiveUI.EditableText_0` (stale `self.ReceiveBeginPlay` _returnvalue_2)) (`KismetTextLibrary.Conv_StringToText` (`KismetStringLibrary.Concat_StrStr` (`self.Begin`) (stale `OnCoreDestroyed_Event` _output_get) (stale `self.ReceiveBeginPlay` _output_get_2))) :!label _label))

(event `OnCoreDestroyed_Event`
  (params (Core :type "BaseCore Object Reference"))
  (`GameplayStatics.SpawnSound2D` "/Game/Audio/SFX/UI/SFX_UI_Objective.SFX_UI_Objective" 1.0 1.0 0.0 null)
  (bind _output_get (set `self.CoresAmount` (`KismetStringLibrary.Conv_IntToString` (- (`KismetArrayLibrary.Array_Length` (`self.Cores`)) 1))))
  (goto _label))

(event `self.ReceiveBeginPlay`
  (bind _returnvalue (`KismetArrayLibrary.Array_Length` (`self.Cores`)))
  (`|ExecutionSequence`
    (:`then_0`
      (bind _returnvalue_2 (`|CreateWidget` "/Game/Interactions/WB_ObjectiveUI.WB_ObjectiveUI_C"))
      (`UserWidget.AddToViewport` _returnvalue_2 0)
      (add `SPMGameInstanceSubsystem.OnCoreDestroyed` (subsystem `SPMGameInstanceSubsystem`) (delegate `OnCoreDestroyed_Event`))
      (bind _output_get (set `self.CoreLength` _returnvalue))
      (set `self.Begin` "Cores To Destoy ")
      (set `self.CoresAmount` (`KismetStringLibrary.Conv_IntToString` _output_get))
      (bind _output_get_2 (set `self.End` (`KismetStringLibrary.Concat_StrStr` " / " (`KismetStringLibrary.Conv_IntToString` _returnvalue))))
      (goto _label))
    (:`then_1`
      (bind _returnvalue_3 (`|CreateWidget` "/Game/Interactions/WB_InteractionPrompt.WB_InteractionPrompt_C"))
      (bind _output_get_3 (set `self.InteractionUserWidget` _returnvalue_3)))))

(fn `UserConstructionScript`)