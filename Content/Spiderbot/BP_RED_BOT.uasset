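; BP_RED_BOT is a bot actor in the Spiderbot folder that takes bonus damage from fireball projectiles.
; On AnyDamage, it compares the damage causer with the single BP_FireballProjectile returned by GetActorOfClass, so only that instance can match.
; A match prints "crit" and applies one extra damage to the bot.
; Every damage event also prints Health's current value minus one as debug output.
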(event `self.ReceiveAnyDamage`
  (params (Damage :type "Float (single-precision)") (DamageType :type "DamageType Object Reference") (InstigatedBy :type "Controller Object Reference") (DamageCauser :type "Actor Object Reference"))
  (bind _returnvalue (`GameplayStatics.GetActorOfClass` "/Game/BP_FireballProjectile.BP_FireballProjectile_C"))
  (if (== _returnvalue DamageCauser)
    (`KismetSystemLibrary.PrintString` "crit")
    (`GameplayStatics.ApplyDamage` self 1.0))
  (`KismetSystemLibrary.PrintString` (`KismetStringLibrary.Conv_DoubleToString` (- (`HealthComponent.GetHealth` (`self.Health`)) 1.0))))

(fn `UserConstructionScript`)