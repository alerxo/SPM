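; BP_Triggerbox_DeactivateDoor is a trigger actor that switches off a set of doors when the player character overlaps it.
; A DoOnce gate limits it to a single firing, which calls Deactivate on every valid entry in DoorsToDeactivate.
; It then destroys the actor referenced by TriggerboxToRemove, if valid, so that other trigger box is removed from the level.
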(event `self.ReceiveActorBeginOverlap`
  (params (OtherActor :type "Actor Object Reference"))
  (bind _triggerboxtoremove (`self.TriggerboxToRemove`))
  ;[1 1 1] Deactivates doors and removes other trigger box if player collides with it
  (if (== OtherActor (`GameplayStatics.GetPlayerCharacter` 0))
    (`/Engine/EditorBlueprintResources/StandardMacros.DoOnce` false
      (:`Completed`
        (`|ExecutionSequence`
          (:`then_0`
            (for _array_element (`self.DoorsToDeactivate`)
              (`/Engine/EditorBlueprintResources/StandardMacros.IsValid` _array_element
                (:`Is Valid`
                  (`/Game/ElectricityDoor/BP_ElectricityDoorUnlock.Deactivate` _array_element)))))
          (:`then_1`
            (`/Engine/EditorBlueprintResources/StandardMacros.IsValid` _triggerboxtoremove
              (:`Is Valid`
                (`self.K2_DestroyActor` _triggerboxtoremove)))))))))

(fn `UserConstructionScript`)