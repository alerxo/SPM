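; Electricity door unlock actor that slides a referenced door open, then closes it automatically after a delay.
; Tick watches CanMove and MoveBack to play open and close timelines, lerping the door between its start location and a leftward/downward offset.
; It swaps its own mesh's emissive locked/unlocked material and plays door sounds.
; After closing, it rewinds the open timeline and, if it is the LevelStreaming subclass, unloads that streamed level.
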(event `self.ReceiveBeginPlay`
  ;[1 1 1] Logic To Get Start Position For Door
  (set `self.Location` (`self.K2_GetActorLocation` (`self.DoorToOpen`)))
  (`PrimitiveComponent.SetMaterial` (`self.GetComponentByClass` self "/Script/Engine.StaticMeshComponent") 0 "/Game/Materials/VFX_Materials/Emissive_Door_Locked.Emissive_Door_Locked"))

(event `self.ReceiveTick`
  (params (DeltaSeconds :type "Float (single-precision)"))
  (bind _doortoopen (`self.DoorToOpen`))
  (bind _returnvalue (- (`self.Location`) (+ (* (`self.GetActorRightVector` _doortoopen) (`self.AmountToMoveLeftward`)) (* (`self.GetActorUpVector` _doortoopen) (`self.AmountToMoveDown`)))))
  (if (and (`self.CanMove`) (not (`self.MoveBack`)))
    ;[1 1 1] Logic To Open The Door
    (bind (_direction _alpha) (`Timeline|Open door` :!label _label)
      (:`Update`
        (`|ExecutionSequence`
          (:`then_0`
            (`self.K2_SetActorRelativeLocation` (`self.DoorToOpen`) (`KismetMathLibrary.VLerp` (`self.Location`) _returnvalue _alpha) false false)
            (`PrimitiveComponent.SetMaterial` (`self.GetComponentByClass` self "/Script/Engine.StaticMeshComponent") 0 "/Game/Materials/VFX_Materials/Emissive_Door_Unlocked.Emissive_Door_Unlocked"))
          (:`then_1`
            (`/Engine/EditorBlueprintResources/StandardMacros.DoOnce` false :!label _label_2
              (:`Completed`
                (`GameplayStatics.PlaySound2D` "/Game/Audio/SFX/Objectives/Doors/SFX_Environment_Door_Open_Close.SFX_Environment_Door_Open_Close" 1.0 1.0 0.0 null null))))))
      (:`Finished`
        (`GameplayStatics.PlaySound2D` "/Game/Audio/SFX/Objectives/Doors/SFX_Environment_Door_Unlock.SFX_Environment_Door_Unlock" 1.0 1.0 0.0 null null)
        (set `self.CanMove` false)
        (`KismetSystemLibrary.Delay` (`self.DoorClosingDelay`))
        (set `self.MoveBack` true)
        (`GameplayStatics.PlaySound2D` "/Game/Audio/SFX/Objectives/Doors/SFX_Environment_Door_Open_Close.SFX_Environment_Door_Open_Close" 1.0 1.0 0.0 null null)
        ;[1 1 1] Logic To Move The Door Back
        (bind (_direction_2 _alpha_2) (`Timeline|Close door` :!via `SetNewTime` :!label _label_3)
          (:`Update`
            (`self.K2_SetActorRelativeLocation` (`self.DoorToOpen`) (`KismetMathLibrary.VLerp` _returnvalue (`self.Location`) _alpha_2) false false))
          (:`Finished`
            (`GameplayStatics.PlaySound2D` "/Game/Audio/SFX/Objectives/Doors/SFX_Environment_Door_Lock.SFX_Environment_Door_Lock" 1.0 1.0 0.0 null null)
            (set `self.MoveBack` false)
            (bind _asbp_electricity_door_unlock_level_streaming (cast `/Game/ElectricityDoor/BP_ElectricityDoorUnlock_LevelStreaming` self)
              (:`then`
                (`/Game/ElectricityDoor/BP_ElectricityDoorUnlock_LevelStreaming.Unload Level Stream` _asbp_electricity_door_unlock_level_streaming))
              (:`CastFailed`
                _))
            (`|ExecutionSequence`
              (:`then_0`
                (goto _label :!via `SetNewTime`))
              (:`then_1`
                (goto _label_2 :!via `Reset`)))))))
    (elif (`self.MoveBack`)
      (goto _label_3)
      (elif (== (`self.K2_GetActorLocation` (`self.DoorToOpen`)) (`self.Location`))
        (`PrimitiveComponent.SetMaterial` (`self.GetComponentByClass` self "/Script/Engine.StaticMeshComponent") 0 "/Game/Materials/VFX_Materials/Emissive_Door_Locked.Emissive_Door_Locked")))))

(fn `UserConstructionScript`)