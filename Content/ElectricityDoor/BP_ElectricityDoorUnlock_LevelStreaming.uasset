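; Electricity door unlock actor that controls level streaming through a referenced streaming volume and can deactivate a linked door.
; It disables the streaming volume on BeginPlay, and separate load and unload events toggle the volume's Disabled flag.
; A DisableDoor event deactivates the referenced door after a validity check.
; Nothing in this graph calls the load or door events, and Tick is unused.
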(event `self.ReceiveBeginPlay`
  (`parent.ReceiveBeginPlay`)
  (`self.Unload Level Stream`))

(event `Load Level Stream`
  (set `LevelStreamingVolume.bDisabled` false (`self.StreamingVolume`)))

(event `Unload Level Stream`
  (set `LevelStreamingVolume.bDisabled` true (`self.StreamingVolume`)))

(event `Disable Door`
  (bind _doortodeactivate (`self.DoorToDeactivate`))
  (`/Engine/EditorBlueprintResources/StandardMacros.IsValid` _doortodeactivate
    (:`Is Valid`
      (`self.Deactivate` _doortodeactivate))))

(fn `UserConstructionScript`
  (`parent.UserConstructionScript`))