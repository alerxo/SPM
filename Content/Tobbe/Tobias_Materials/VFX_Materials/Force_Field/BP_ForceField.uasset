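; BP_ForceField is a force field actor that animates its mesh material through timelines.
; ShowForceField plays an alpha timeline into the "Alpha" parameter, then on finish calls HideForceField to reverse it and immediately destroys the actor.
; Hits on the ForceField component restart a Bounce timeline, sped up at BeginPlay, that drives "Bounce Alpha".
; Nothing in this graph triggers ShowForceField, as its only call is disconnected.
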(event `self.ReceiveBeginPlay`
  (`TimelineComponent.SetPlayRate` (`self.Bounce`) 3.0))

(event `ShowForceField`
  (bind (_direction _alpha) (`Timeline|Animate_Alpha` :!label _label)
    (:`Update`
      (`MeshComponent.SetScalarParameterValueOnMaterials` (`self.ForceField`) "Alpha" _alpha))
    (:`Finished`
      (`self.HideForceField`)
      (`self.K2_DestroyActor`))))

(event `HideForceField`
  (goto _label :!via `Reverse`))

(event `self.ForceField.OnComponentHit`
  (params (HitComponent :type "PrimitiveComponent Object Reference") (OtherActor :type "Actor Object Reference") (OtherComp :type "PrimitiveComponent Object Reference") (NormalImpulse :type "Vector Structure") (Hit :type "HitResult Structure (by ref)"))
  (bind (_direction _bounce_alpha) (`Timeline|Bounce` :!via `PlayFromStart`)
    (:`Update`
      (`MeshComponent.SetScalarParameterValueOnMaterials` (`self.ForceField`) "Bounce Alpha" _bounce_alpha))))

(fn `UserConstructionScript`)