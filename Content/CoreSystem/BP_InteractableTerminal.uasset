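; Interactable terminal linked to a BP_Core that handles temporarily lowering its shield, with an interaction prompt on sphere overlap.
; On disable, it drops force-field collision, enables core damage and hides the prompt, while Tick counts down to reactivation, which restores these and reduces the MasterMind token limit.
; Timelines fade the force-field material, both transitions update the player's objective, and Tick shows core health and countdown while the player is nearby.
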(event `OnCoreReactivated`
  (bind _spherecomponent (`self.SphereComponent`))
  (bind _core (`self.Core`))
  ;[1 1 1] När coren ska activeras igen så ändra de nödvändiga sakerna
  (`|ExecutionSequence`
    (:`then_0`
      (set `self.ShowCoreHealth` false))
    (:`then_1`
      (`PrimitiveComponent.SetMaterial` (`self.MeshComponent`) 1 "/Game/Materials/Tobias_Materials/VFX_Materials/Emissive_Materials/Emissive_Health.Emissive_Health")
      (`|ExecutionSequence`
        (:`then_0`
          (add `PrimitiveComponent.OnComponentBeginOverlap` _spherecomponent (delegate `OnComponentBeginOverlap`))
          (add `PrimitiveComponent.OnComponentEndOverlap` _spherecomponent (delegate `OnComponentEndOvelap`)))
        (:`then_1`
          ;;[0 1 0.01725] Updates The objective UI
          (bind _asbp_first_person_character (cast `/Game/FirstPerson/Blueprints/BP_FirstPersonCharacter` (`GameplayStatics.GetPlayerCharacter` 0)))
          (bind _stepbystepobjective (`/Game/FirstPerson/Blueprints/BP_FirstPersonCharacter.StepByStepObjective` _asbp_first_person_character))
          (bind _fadeout (`/Game/UI/Objectives/StepByStepMissions/WB_StepByStepObjective.FadeOut` _stepbystepobjective))
          (if (not (`UserWidget.IsAnimationPlaying` _stepbystepobjective _fadeout))
            (`UserWidget.PlayAnimation` _stepbystepobjective _fadeout 0.0 1 "Forward" 1.0 false)
            (`KismetSystemLibrary.Delay` 0.5)
            (`/Game/FirstPerson/Blueprints/BP_FirstPersonCharacter.UpdateObjective` _asbp_first_person_character (`self.CoreShieldActive`) (`self.DetailedCoreShieldActive`))
            (bind _fadein (`/Game/UI/Objectives/StepByStepMissions/WB_StepByStepObjective.FadeIn` _stepbystepobjective))
            (if (not (`UserWidget.IsAnimationPlaying` _stepbystepobjective _fadein))
              (`UserWidget.PlayAnimation` _stepbystepobjective _fadein 0.0 1 "Forward" 1.0 false)
              (`KismetSystemLibrary.Delay` 1.2))))
        (:`then_2`
          (`/Engine/EditorBlueprintResources/StandardMacros.IsValid` _core
            (:`Is Valid`
              (bind _asbp_core (cast `/Game/CoreSystem/BP_Core` _core))
              (`/Engine/EditorBlueprintResources/StandardMacros.IsValid` _asbp_core
                (:`Is Valid`
                  (`GameplayStatics.PlaySound2D` "/Game/Audio/SFX/Objectives/Core/SFX_Objective_Core_Shield_Activate.SFX_Objective_Core_Shield_Activate" 1.0 1.0 0.0 null null)
                  (`PrimitiveComponent.SetCollisionEnabled` (`/Game/CoreSystem/BP_Core.ForceFieldCollision` _asbp_core) "QueryAndPhysics")
                  (set `self.ShowCoreHealth` false)
                  (`AudioComponent.Play` (`/Game/CoreSystem/BP_Core.Audio` _asbp_core) 0.0)
                  (`HealthComponent.DisableTakeDamage` (`BaseCore.HealthComponent` _asbp_core))
                  (`SPMGameInstanceSubsystem.OnCoreActivated` (subsystem `SPMGameInstanceSubsystem`) (`self.Core`)))))))
        (:`then_3`
          (bind _forcefield (`/Game/CoreSystem/BP_Core.ForceField` _asbp_core))
          ;;[0.01177 0.698 1] Timeline Node to Animate the reactivation of the Force Field
          (`MeshComponent.SetScalarParameterValueOnMaterials` _forcefield "Alpha" 1.0)
          (bind (_direction _alpha) (`Timeline|Timeline_1` :!via `ReverseFromEnd`)
            (:`Update`
              (`/Engine/EditorBlueprintResources/StandardMacros.IsValid` _forcefield
                (:`Is Valid`
                  (`MeshComponent.SetScalarParameterValueOnMaterials` _forcefield "Alpha" _alpha))))))))
    (:`then_2`
      (`MasterMindInstancedSubsystem.ReduceTokenLimit` (subsystem `MasterMindInstancedSubsystem`) 1.0))))

(event `OnCoreDeactivated_Event`
  (bind _spherecomponent (`self.SphereComponent`))
  (bind _core (`self.Core`))
  ;[1 1 1] När coren ska bli deactiverad så körs detta
  (`|ExecutionSequence`
    (:`then_0`
      (`PrimitiveComponent.SetMaterial` (`self.MeshComponent`) 1 "/Game/Materials/Tobias_Materials/VFX_Materials/Emissive_Materials/_Tutorial._Tutorial")
      (set `self.IsShieldDown` true)
      (`|ExecutionSequence`
        (:`then_0`
          (remove `PrimitiveComponent.OnComponentBeginOverlap` _spherecomponent (delegate `OnComponentBeginOverlap`))
          (remove `PrimitiveComponent.OnComponentEndOverlap` _spherecomponent (delegate `OnComponentEndOvelap`))
          (`Widget.RemoveFromParent` (`self.UserWidget`)))
        (:`then_1`
          (`/Engine/EditorBlueprintResources/StandardMacros.IsValid` _core
            (:`Is Valid`
              (bind _asbp_core (cast `/Game/CoreSystem/BP_Core` _core))
              (`PrimitiveComponent.SetCollisionEnabled` (`/Game/CoreSystem/BP_Core.ForceFieldCollision` _asbp_core) "NoCollision")
              (bind _asbp_first_person_character (cast `/Game/FirstPerson/Blueprints/BP_FirstPersonCharacter` (`GameplayStatics.GetPlayerCharacter` 0)))
              (bind _stepbystepobjective (`/Game/FirstPerson/Blueprints/BP_FirstPersonCharacter.StepByStepObjective` _asbp_first_person_character))
              (bind _fadeout (`/Game/UI/Objectives/StepByStepMissions/WB_StepByStepObjective.FadeOut` _stepbystepobjective))
              (if (not (`UserWidget.IsAnimationPlaying` _stepbystepobjective _fadeout))
                (`UserWidget.PlayAnimation` _stepbystepobjective _fadeout 0.0 1 "Forward" 1.0 false)
                (`KismetSystemLibrary.Delay` 0.5)
                (`/Game/FirstPerson/Blueprints/BP_FirstPersonCharacter.UpdateObjective` _asbp_first_person_character (`self.CoreShieldDisabled`) (`self.DetailedCoreShieldDisabled`))
                (bind _fadein (`/Game/UI/Objectives/StepByStepMissions/WB_StepByStepObjective.FadeIn` _stepbystepobjective))
                (if (not (`UserWidget.IsAnimationPlaying` _stepbystepobjective _fadein))
                  (`UserWidget.PlayAnimation` _stepbystepobjective _fadein 0.0 1 "Forward" 1.0 false)
                  (`KismetSystemLibrary.Delay` 1.2))))))
        (:`then_2`
          (`HealthComponent.ActivateTakeDamage` (`BaseCore.HealthComponent` _asbp_core))
          (set `self.ShowCoreHealth` true)
          (`GameplayStatics.PlaySound2D` "/Game/Audio/SFX/Objectives/Core/SFX_Objective_Core_Shield_Deactivate.SFX_Objective_Core_Shield_Deactivate" 1.0 1.0 0.0 null null)
          (`AudioComponent.Stop` (`/Game/CoreSystem/BP_Core.Audio` _asbp_core))
          (`SPMGameInstanceSubsystem.OnCoreDeactivated` (subsystem `SPMGameInstanceSubsystem`) (`self.Core`)))))
    (:`then_1`
      (bind _asbp_core_2 (cast `/Game/CoreSystem/BP_Core` (`self.Core`)))
      ;;[0.01177 0.698 1] Play Timeline to deactivate the ForceField
      (bind (_direction _alpha) (`Timeline|Timeline` :!via `PlayFromStart`)
        (:`Update`
          (bind _forcefield (`/Game/CoreSystem/BP_Core.ForceField` _asbp_core_2))
          (`/Engine/EditorBlueprintResources/StandardMacros.IsValid` _forcefield
            (:`Is Valid`
              (`MeshComponent.SetScalarParameterValueOnMaterials` _forcefield "Alpha" _alpha))))))))

(event `CoreDestroyed`
  (params (Core :type "BaseCore Object Reference"))
  ;[1 1 1] When Core is Destroyed
  (bind _asbp_core (cast `/Game/CoreSystem/BP_Core` Core))
  (bind _cable (`/Game/CoreSystem/BP_Core.Cable` _asbp_core))
  (`/Engine/EditorBlueprintResources/StandardMacros.IsValid` _cable
    (:`Is Valid`
      (`self.K2_DestroyActor` _cable))))

(event `OnDead_Event`
  ;[1 1 1] When The core is Dead
  (set `self.IsCoreDead` true)
  (`self.SetActorTickEnabled` false))

(event `OnComponentEndOvelap`
  (params (OverlappedComponent :type "PrimitiveComponent Object Reference") (OtherActor :type "Actor Object Reference") (OtherComp :type "PrimitiveComponent Object Reference") (OtherBodyIndex :type Integer))
  ;[1 1 1] Overlapping Events
  (`Widget.RemoveFromParent` (`self.UserWidget`)))

(event `OnComponentBeginOverlap`
  (params (OverlappedComponent :type "PrimitiveComponent Object Reference") (OtherActor :type "Actor Object Reference") (OtherComp :type "PrimitiveComponent Object Reference") (OtherBodyIndex :type Integer) (bFromSweep :type Boolean) (SweepResult :type "HitResult Structure (by ref)"))
  ;[1 1 1] Overlapping Events
  (`UserWidget.AddToViewport` (`self.UserWidget`) 0))

(event `self.ReceiveBeginPlay`
  (bind _spherecomponent (`self.SphereComponent`))
  ;[1 1 1] Begin Play sets events and diffretn Variables
  (bind _returnvalue (`|CreateWidget` "/Game/Interactions/WB_InteractionPrompt.WB_InteractionPrompt_C"))
  (set `self.UserWidget` _returnvalue)
  (add `self.OnCoreDisabled` (delegate `OnCoreDeactivated_Event`))
  (add `self.OnCoreReActive` (delegate `OnCoreReactivated`))
  (add `PrimitiveComponent.OnComponentBeginOverlap` _spherecomponent (delegate `OnComponentBeginOverlap`))
  (add `PrimitiveComponent.OnComponentEndOverlap` _spherecomponent (delegate `OnComponentEndOvelap`))
  (add `SPMGameInstanceSubsystem.OnCoreDestroyed` (subsystem `SPMGameInstanceSubsystem`) (delegate `CoreDestroyed`))
  (add `HealthComponent.OnDead` (`BaseCore.HealthComponent` (`self.Core`)) (delegate `OnDead_Event`))
  (set `self.Timer` (`self.DefaultTimer`))
  (set `self.SPMSubSytem` self))

(event `self.ReceiveTick`
  (params (DeltaSeconds :type "Float (single-precision)"))
  (bind _core (`self.Core`))
  ;[1 1 1] Tick för att utföra en timer när corens sköld ska aktiveras
  (`|ExecutionSequence`
    (:`then_0`
      (if (`self.IsShieldDown`)
        (bind _output_get (set `self.Timer` (- (`self.Timer`) DeltaSeconds)))
        (if (<= _output_get 0.0)
          (`KismetSystemLibrary.PrintString` "CALL RE ACTUVE")
          (set `self.Timer` (`self.DefaultTimer`))
          (set `self.IsShieldDown` false)
          (`self.OnCoreReActive`))))
    (:`then_1`
      (if (not (`self.IsCoreDead`))
        (`/Engine/EditorBlueprintResources/StandardMacros.IsValid` _core
          (:`Is Valid`
            (bind _asbp_core (cast `/Game/CoreSystem/BP_Core` _core))
            (`|ExecutionSequence`
              (:`then_0`
                (bind _returnvalue (`self.Should Show Core Health` _asbp_core))
                (bind _corehealthwidget (`/Game/CoreSystem/BP_Core.CoreHealthWidget` _asbp_core))
                (`/Engine/EditorBlueprintResources/StandardMacros.IsValid` _corehealthwidget
                  (:`Is Valid`
                    (`self.ShieldTimerText` (`/Game/UI/WB_CoreHealth.ShieldTimer` _corehealthwidget))
                    (if (and (`self.ShowCoreHealth`) _returnvalue)
                      (`Widget.SetVisibility` _corehealthwidget "Visible")
                      (else
                        (`Widget.SetVisibility` _corehealthwidget "Hidden")))))))))))))

(fn `GetCoreLength`
  (returns (CoreLength :type Integer))
  (bind _outactors (`GameplayStatics.GetAllActorsOfClass` "/Game/CoreSystem/BP_Core.BP_Core_C"))
  (return (`KismetArrayLibrary.Array_Length` _outactors)))

(fn `ShieldTimerText`
  (params (`Shield Timer` :type "TextBlock Object Reference"))
  (set `TextBlock.Text` (`KismetTextLibrary.Conv_StringToText` (`KismetStringLibrary.Concat_StrStr` (`self.TimerText`) (`KismetStringLibrary.Conv_Int64ToString` (`KismetMathLibrary.Conv_DoubleToInt64` (`self.Timer`))) "s")) `Shield Timer`))

(fn `Should Show Core Health`
  (params (Core :type "/Game/CoreSystem/BP_Core Object Reference"))
  (returns (ReturnValue :type Boolean))
  (return (and (`PrimitiveComponent.IsOverlappingActor` (`/Game/CoreSystem/BP_Core.CoreHealthCollider` Core) (`GameplayStatics.GetPlayerCharacter` 0)) (>= (`HealthComponent.GetHealth` (`self.GetComponentByClass` Core "/Script/SPM.HealthComponent")) 0.0))))

(fn `UserConstructionScript`)