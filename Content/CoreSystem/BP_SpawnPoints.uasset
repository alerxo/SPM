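; BP_SpawnPoints is a destructible spawn location actor with a Health component, which has damage disabled on BeginPlay.
; Any damage event runs Checkhealth, which removes the actor from its Spawner's SpawnLocations and destroys it once health reaches zero or below.
; The graph that would fetch Spawner from BP_MasterMind is disconnected, so this Blueprint never assigns that reference itself.
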(event `self.ReceiveBeginPlay`
  (add `self.OnTakeAnyDamage` (delegate `OnTakeDamageEvent`))
  (`HealthComponent.DisableTakeDamage` (`self.Health`)))

(event `OnTakeDamageEvent` :!signature `self.OnTakeAnyDamage`
  (params (DamagedActor :type "Actor Object Reference") (Damage :type "Float (single-precision)") (DamageType :type "DamageType Object Reference") (InstigatedBy :type "Controller Object Reference") (DamageCauser :type "Actor Object Reference"))
  (`self.Checkhealth`))

(fn `Checkhealth`
  (if (<= (`HealthComponent.GetHealth` (`self.Health`)) 0.0)
    (`KismetArrayLibrary.Array_RemoveItem` (`Spawner.SpawnLocations` (`self.Spawner`)) self)
    (`self.K2_DestroyActor`))
  (return))

(fn `UserConstructionScript`)