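; Destructible core objective that starts damage-immune with a hidden health widget and emits sparks once when health drops below a threshold.
; On death it explodes with camera shake, teleports to a fixed location, saves a checkpoint with a notification, lowers the MasterMind token limit, activates linked electricity doors and updates the player's objective.
; A separate Destroyed handler repeats the widget cleanup and explosion, and records the destroyed object with the GameMode.
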(event `self.ReceiveBeginPlay`
  (bind _returnvalue (`|CreateWidget` "/Game/UI/WB_CoreHealth.WB_CoreHealth_C" (`GameplayStatics.GetPlayerController` 0)))
  (bind _output_get (set `self.CoreHealthWidget` _returnvalue))
  (`UserWidget.AddToViewport` _output_get 0)
  (`Widget.SetVisibility` _output_get "Hidden")
  (`HealthComponent.DisableTakeDamage` (`self.HealthComponent`)))

(event `self.ReceiveDestroyed`
  (`|ExecutionSequence`
    (:`then_0`
      (`Widget.RemoveFromParent` (`self.CoreHealthWidget`))
      (set `self.CoreHealthWidget` null))
    (:`then_1`
      (`NiagaraFunctionLibrary.SpawnSystemAtLocation` "/Game/Particle/Explosion/Explosion.Explosion" (`self.K2_GetActorLocation` self) (`self.K2_GetActorRotation` self))
      (`LegacyCameraShake.StartLegacyCameraShake` null "/Script/GameplayCameras.LegacyCameraShake" 10.0))
    (:`then_2`
      (message `/Game/SaveSystem/BPI_SaveObjects.SaveDestroyedObject` (`GameplayStatics.GetGameMode`) self))))

(event `self.ReceiveTick`
  (params (DeltaSeconds :type "Float (single-precision)"))
  ;[1 1 1] Ligger på IS
  (`|ExecutionSequence`
    (:`then_1`
      (if (and (`self.CanPlay`) (< (`HealthComponent.GetHealthPercentage` (`self.GetComponentByClass` self "/Script/SPM.HealthComponent")) (`self.Percentage`)))
        (`NiagaraFunctionLibrary.SpawnSystemAttached` "/Game/Particle/NG_Sparks1.NG_Sparks1" null "None" (`self.K2_GetActorLocation` self) (`self.K2_GetActorRotation` self) "KeepWorldPosition")
        (set `self.CanPlay` false)))))

(event `self.HealthComponent.OnDead`
  (bind _electricitydoorstoactivate (`self.ElectricityDoorsToActivate`))
  (`self.DestroyCore`)
  (`|ExecutionSequence`
    (:`then_0`
      (`Widget.RemoveFromParent` (`self.CoreHealthWidget`))
      (set `self.CoreHealthWidget` null))
    (:`then_1`
      (`NiagaraFunctionLibrary.SpawnSystemAtLocation` "/Game/Particle/Explosion/Explosion.Explosion" (`self.K2_GetActorLocation` self) (`self.K2_GetActorRotation` self))
      (`GameplayStatics.PlayWorldCameraShake` "/Game/CoreSystem/CoreCameraShake.CoreCameraShake_C" (`self.K2_GetActorLocation`) 0.0 2000.0 1.0 true)
      (`self.K2_SetActorLocation` (7225.0 -15010.0 -1225.0) false true))
    (:`then_2`
      ;[1 1 1] Save game as a checkpoint
      (`self.SaveGameState`)
      (bind _returnvalue (`|CreateWidget` "/Game/UI/WB_CheckpointReached.WB_CheckpointReached_C"))
      (`UserWidget.AddToViewport` _returnvalue 0)
      (`GameplayStatics.PlaySound2D` "/Game/Audio/SFX/UI/SFX_UI_Objective.SFX_UI_Objective" 1.0 1.0 0.0 null null)
      (`UserWidget.PlayAnimation` _returnvalue (`/Game/UI/WB_CheckpointReached.CheckpointReached` _returnvalue) 0.0 1 "Forward" 1.0 false)
      (`KismetSystemLibrary.Delay` 2.6)
      (`Widget.RemoveFromParent` _returnvalue))
    (:`then_3`
      (`MasterMindInstancedSubsystem.ReduceTokenLimit` (subsystem `MasterMindInstancedSubsystem`) 1.0))
    (:`then_4`
      ;[1 1 1] Activates doors
      (if (not (`KismetArrayLibrary.Array_IsEmpty` _electricitydoorstoactivate))
        (for _array_element _electricitydoorstoactivate
          (`/Engine/EditorBlueprintResources/StandardMacros.IsValid` _array_element
            (:`Is Valid`
              (`/Game/ElectricityDoor/BP_ElectricityDoorUnlock.Activate` _array_element))))))
    (:`then_5`
      (bind _asbp_first_person_character (cast `/Game/FirstPerson/Blueprints/BP_FirstPersonCharacter` (`GameplayStatics.GetPlayerCharacter` 0)))
      (bind _stepbystepobjective (`/Game/FirstPerson/Blueprints/BP_FirstPersonCharacter.StepByStepObjective` _asbp_first_person_character))
      (`UserWidget.PlayAnimation` _stepbystepobjective (`/Game/UI/Objectives/StepByStepMissions/WB_StepByStepObjective.FadeOut` _stepbystepobjective) 0.0 1 "Forward" 1.0 false)
      (`KismetSystemLibrary.Delay` 0.5)
      (`/Game/FirstPerson/Blueprints/BP_FirstPersonCharacter.UpdateObjective` _asbp_first_person_character (`self.New Objective`) (`self.Details`))
      (`UserWidget.PlayAnimation` _stepbystepobjective (`/Game/UI/Objectives/StepByStepMissions/WB_StepByStepObjective.FadeIn` _stepbystepobjective) 0.0 1 "Forward" 1.0 false)
      (`KismetSystemLibrary.Delay` 1.2)
      (`self.ClearVariables`))))

(fn `ClearVariables`
  (set `self.Percentage` 0.0)
  (set `self.CoreHealthWidget` null)
  (set `self.ShieldDoor` null)
  (set `self.New Objective` "")
  (set `self.Details` "")
  (`KismetArrayLibrary.Array_Clear` (`self.ElectricityDoorsToActivate`)))

(fn `SaveGameState`
  (bind _returnvalue (`GameplayStatics.GetGameMode`))
  (bind _returnvalue_2 (`GameplayStatics.GetPlayerCharacter` 0))
  ;[1 1 1] Save game (checkpoint) after every destroyed core
  (message `/Game/SaveSystem/BPI_SaveObjects.SaveDestroyedObject` _returnvalue self)
  (message `/Game/SaveSystem/BPI_SaveObjects.SavePlayerHealth` _returnvalue)
  (message `/Game/SaveSystem/BPI_SaveObjects.SavePlayerPosition` _returnvalue (`self.K2_GetActorLocation` _returnvalue_2) (`self.K2_GetActorRotation` _returnvalue_2))
  (message `/Game/SaveSystem/BPI_SaveObjects.SaveGame` (`GameplayStatics.GetGameMode`)))

(fn `UserConstructionScript`)