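; Core terminal that shows an interaction prompt while active and tracks the cores left to destroy on the player's objective HUD.
; The subsystem's core-destroyed event plays a sound, updates the counter and, a tick later, fades in a new step objective, distinguishing the last core.
; It also removes the core from its shield door's list and triggers that door's deactivation check.
; An OnSave binding forwards zeroed player transform values and a save request to the GameMode.
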(event `self.SphereComponent.OnComponentBeginOverlap`
  (params (OverlappedComponent :type "PrimitiveComponent Object Reference") (OtherActor :type "Actor Object Reference") (OtherComp :type "PrimitiveComponent Object Reference") (OtherBodyIndex :type Integer) (bFromSweep :type Boolean) (SweepResult :type "HitResult Structure (by ref)"))
  ;[1 1 1] Overlapping Event
  (if (`self.bIsActive`)
    (`UserWidget.AddToViewport` (stale `self.ReceiveBeginPlay` _output_get) 0)))

(event `self.SphereComponent.OnComponentEndOverlap`
  (params (OverlappedComponent :type "PrimitiveComponent Object Reference") (OtherActor :type "Actor Object Reference") (OtherComp :type "PrimitiveComponent Object Reference") (OtherBodyIndex :type Integer))
  ;[1 1 1] Overlapping Event
  (`Widget.RemoveFromParent` (stale `self.ReceiveBeginPlay` _output_get)))

(event `SavePlayerPosition`
  (bind _returnvalue (`GameplayStatics.GetGameMode`))
  ;[1 1 1] Save Player Position
  (message `/Game/SaveSystem/BPI_SaveObjects.SavePlayerPosition` _returnvalue (0.0 0.0 0.0) (struct))
  (message `/Game/SaveSystem/BPI_SaveObjects.SaveGame` _returnvalue))

(event `self.ReceiveBeginPlay`
  (bind _returnvalue (`KismetArrayLibrary.Array_Length` (`self.Cores`)))
  ;[1 1 1] Begin Event
  (`|ExecutionSequence`
    (:`then_0`
      (add `self.OnSave` (delegate `SavePlayerPosition`)))
    (:`then_1`
      (bind _returnvalue_2 (`|CreateWidget` "/Game/Interactions/WB_InteractionPrompt.WB_InteractionPrompt_C"))
      (bind _output_get (set `self.InteractionUserWidget` _returnvalue_2)))
    (:`then_2`
      (add `SPMGameInstanceSubsystem.OnCoreDestroyed` (subsystem `SPMGameInstanceSubsystem`) (delegate `OnCoreDestroyed_Event`))
      (`KismetSystemLibrary.DelayUntilNextTick`)
      (bind _asbp_first_person_character (cast `/Game/FirstPerson/Blueprints/BP_FirstPersonCharacter` (`GameplayStatics.GetPlayerCharacter` 0)))
      (bind _output_get_2 (set `self.CoreLength` _returnvalue))
      (set `self.Begin` "Cores Left: ")
      (set `self.CoresAmount` (`KismetStringLibrary.Conv_IntToString` _output_get_2))
      (set `self.End` (`KismetStringLibrary.Concat_StrStr` " / " (`KismetStringLibrary.Conv_IntToString` _returnvalue)))
      (`EditableText.SetText` (`/Game/UI/WB_ObjectiveUI.EditableText_0` (`/Game/FirstPerson/Blueprints/BP_FirstPersonCharacter.Main Objective` _asbp_first_person_character)) (`KismetTextLibrary.Conv_StringToText` (`KismetStringLibrary.Concat_StrStr` (`self.Begin`) (stale `OnCoreDestroyed_Event` _output_get))) :!label _label))))

(event `OnCoreDestroyed_Event`
  (params (Core :type "BaseCore Object Reference"))
  (bind _returnvalue (`GameplayStatics.GetPlayerCharacter` 0))
  (bind _cores (`self.Cores`))
  ;[1 1 1] Whhen the Core is Desstroyed
  (`|ExecutionSequence`
    (:`then_0`
      (`GameplayStatics.SpawnSound2D` "/Game/Audio/SFX/UI/SFX_UI_Objective.SFX_UI_Objective" 1.0 1.0 0.0 null)
      (bind _output_get (set `self.CoresAmount` (`KismetStringLibrary.Conv_IntToString` (- (`KismetArrayLibrary.Array_Length` _cores) 1))))
      (goto _label))
    (:`then_1`
      (`KismetSystemLibrary.DelayUntilNextTick`)
      (if (`KismetArrayLibrary.Array_IsEmpty` _cores)
        (bind _asbp_first_person_character (cast `/Game/FirstPerson/Blueprints/BP_FirstPersonCharacter` _returnvalue))
        (bind _stepbystepobjective (`/Game/FirstPerson/Blueprints/BP_FirstPersonCharacter.StepByStepObjective` _asbp_first_person_character))
        (bind _fadeout (`/Game/UI/Objectives/StepByStepMissions/WB_StepByStepObjective.FadeOut` _stepbystepobjective))
        (if (not (`UserWidget.IsAnimationPlaying` _stepbystepobjective _fadeout))
          (`UserWidget.PlayAnimation` _stepbystepobjective _fadeout 0.0 1 "Forward" 1.0 false)
          (`KismetSystemLibrary.Delay` 0.5)
          (`/Game/FirstPerson/Blueprints/BP_FirstPersonCharacter.UpdateObjective` _asbp_first_person_character (`self.On Last Core Destroyed Objective`) "")
          (bind _fadein (`/Game/UI/Objectives/StepByStepMissions/WB_StepByStepObjective.FadeIn` _stepbystepobjective))
          (if (not (`UserWidget.IsAnimationPlaying` _stepbystepobjective _fadein))
            (`UserWidget.PlayAnimation` _stepbystepobjective _fadein 0.0 1 "Forward" 1.0 false)
            (`KismetSystemLibrary.Delay` 1.2 :!label _label_2)))
        (else
          (bind _asbp_first_person_character_2 (cast `/Game/FirstPerson/Blueprints/BP_FirstPersonCharacter` _returnvalue))
          (bind _stepbystepobjective_2 (`/Game/FirstPerson/Blueprints/BP_FirstPersonCharacter.StepByStepObjective` _asbp_first_person_character_2))
          (bind _fadeout_2 (`/Game/UI/Objectives/StepByStepMissions/WB_StepByStepObjective.FadeOut` _stepbystepobjective_2))
          (if (not (`UserWidget.IsAnimationPlaying` _stepbystepobjective_2 _fadeout_2))
            (`UserWidget.PlayAnimation` _stepbystepobjective_2 _fadeout_2 0.0 1 "Forward" 1.0 false)
            (`KismetSystemLibrary.Delay` 0.5)
            (`/Game/FirstPerson/Blueprints/BP_FirstPersonCharacter.UpdateObjective` _asbp_first_person_character_2 (`self.On Core Destroyed Objective`) "")
            (bind _fadein_2 (`/Game/UI/Objectives/StepByStepMissions/WB_StepByStepObjective.FadeIn` _stepbystepobjective_2))
            (if (not (`UserWidget.IsAnimationPlaying` _stepbystepobjective_2 _fadein_2))
              (`UserWidget.PlayAnimation` _stepbystepobjective_2 _fadein_2 0.0 1 "Forward" 1.0 false)
              (goto _label_2))))))
    (:`then_2`
      (bind _asbp_core (cast `/Game/CoreSystem/BP_Core` Core))
      (bind _shielddoor (`/Game/CoreSystem/BP_Core.ShieldDoor` _asbp_core))
      (`/Engine/EditorBlueprintResources/StandardMacros.IsValid` _shielddoor
        (:`Is Valid`
          (`KismetArrayLibrary.Array_RemoveItem` (`/Game/BP_Shield_Door.CoresToDeactivateDoor` _shielddoor) _asbp_core)
          (`/Game/BP_Shield_Door.CheckToDeactivate` _shielddoor))))))

(fn `UserConstructionScript`)