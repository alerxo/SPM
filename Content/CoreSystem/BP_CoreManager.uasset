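; BP_CoreManager opens the way through a door's force field once all cores are destroyed.
; On BeginPlay it binds a handler to the all-cores-destroyed event.
; The handler plays a shield deactivation sound and runs a Timeline that drives the force field material's Alpha parameter, then disables its collision when finished.
; An unconnected node that would hide the door never runs.
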(event `OnAllCoresDestroyed`
  (bind _forcefield (`/Game/CoreSystem/Door.ForceField` (`self.Door`)))
  (`GameplayStatics.PlaySound2D` "/Game/Audio/SFX/Objectives/Core/SFX_Objective_Core_Shield_Deactivate.SFX_Objective_Core_Shield_Deactivate" 1.0 1.0 0.0 null null)
  (bind (_direction _alpha) (`Timeline|Timeline`)
    (:`Update`
      (`MeshComponent.SetScalarParameterValueOnMaterials` _forcefield "Alpha" _alpha))
    (:`Finished`
      (`PrimitiveComponent.SetCollisionEnabled` _forcefield "NoCollision"))))

(event `self.ReceiveBeginPlay`
  (add `self.OnAllCoresDestroy` (delegate `OnAllCoresDestroyed`)))

(event `self.ReceiveTick`
  (params (DeltaSeconds :type "Float (single-precision)")))

(fn `UserConstructionScript`)