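; BP_Shield_Door is a shield door that dissolves and removes itself once its list of required cores is empty.
; CheckToDeactivate tests CoresToDeactivateDoor, which this graph never edits, and plays the DeactivateShield timeline when none remain.
; The timeline drives the mesh material's Alpha parameter, plays a deactivation sound once through a DoOnce, and destroys the actor when finished.
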(event `CheckToDeactivate`
  (if (`KismetArrayLibrary.Array_IsEmpty` (`self.CoresToDeactivateDoor`))
    (bind (_direction _newtrack_0) (`Timeline|DeactivateShield` :!label _label)
      (:`Update`
        (`|ExecutionSequence`
          (:`then_0`
            (`/Engine/EditorBlueprintResources/StandardMacros.IsValid` self
              (:`Is Valid`
                (`MeshComponent.SetScalarParameterValueOnMaterials` (`self.StaticMeshComponent`) "Alpha" _newtrack_0))
              (:`Is Not Valid`
                (goto _label :!via `Stop`))))
          (:`then_1`
            (`/Engine/EditorBlueprintResources/StandardMacros.DoOnce` false
              (:`Completed`
                (`GameplayStatics.PlaySoundAtLocation` "/Game/Audio/SFX/Objectives/Core/SFX_Objective_Core_Shield_Deactivate.SFX_Objective_Core_Shield_Deactivate" (`self.K2_GetActorLocation`) (struct) 1.0 1.0 0.0 null null null null))))))
      (:`Finished`
        (`self.K2_DestroyActor`)))))

(fn `UserConstructionScript`)