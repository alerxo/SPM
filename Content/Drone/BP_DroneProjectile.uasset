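; BP_DroneProjectile is a projectile that homes in on the first player's pawn and damages whatever it hits.
; BeginPlay targets a scene component on that pawn and turns on very strong homing through the ProjectileMovementComponent.
; Tick permanently switches homing off once the projectile is too far from the pawn.
; When the projectile stops, it applies its Damage to the hit actor and destroys itself.
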(event `self.ReceiveBeginPlay`
  (bind _returnvalue (`self.GetComponentByClass` self "/Script/Engine.ProjectileMovementComponent"))
  (set `ProjectileMovementComponent.HomingTargetComponent` (`self.GetComponentByClass` (`GameplayStatics.GetPlayerPawn` 0) "/Script/Engine.SceneComponent") _returnvalue)
  (set `ProjectileMovementComponent.bIsHomingProjectile` true _returnvalue)
  (set `ProjectileMovementComponent.HomingAccelerationMagnitude` 10000000.0 _returnvalue))

(event `self.ReceiveTick`
  (params (DeltaSeconds :type "Float (single-precision)"))
  (if (not (< (`KismetMathLibrary.Vector_Distance` (`self.K2_GetActorLocation` self) (`self.K2_GetActorLocation` (`GameplayStatics.GetPlayerPawn` 0))) 10000.0))
    (set `ProjectileMovementComponent.bIsHomingProjectile` false (`self.GetComponentByClass` self "/Script/Engine.ProjectileMovementComponent"))))

(event `self.ProjectileMovement.OnProjectileStop`
  (params (ImpactResult :type "HitResult Structure (by ref)"))
  (`GameplayStatics.ApplyDamage` (`.HitActor` (`GameplayStatics.BreakHitResult` ImpactResult)) (`self.Damage`) null self)
  (`self.K2_DestroyActor` self))

(fn `UserConstructionScript`)