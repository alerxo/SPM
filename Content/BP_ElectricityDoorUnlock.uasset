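; BP_ElectricityDoorUnlock slides a referenced door actor open along its negative right vector, then closes it after a delay.
; Tick polls the CanMove flag, which nothing here sets true, to play the OpenDoor timeline.
; When that finishes, a three-second pause sets MoveBack, so Tick plays CloseDoor, and both timelines are rewound during the cycle.
; Both lerp from the world location cached at BeginPlay but apply it as relative location.
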(event `self.ReceiveBeginPlay`
  (set `self.Location` (`self.K2_GetActorLocation` (`self.DoorToOpen`))))

(event `self.ReceiveTick`
  (params (DeltaSeconds :type "Float (single-precision)"))
  (bind _doortoopen (`self.DoorToOpen`))
  (bind _location (`self.Location`))
  (bind _returnvalue (- _location (* (`self.GetActorRightVector` _doortoopen) (`self.Amount To Move`))))
  (if (and (`self.CanMove`) (not (`self.MoveBack`)))
    (bind (_direction _alpha) (`Timeline|Open door` :!label _label)
      (:`Update`
        (`self.K2_SetActorRelativeLocation` _doortoopen (`KismetMathLibrary.VLerp` _location _returnvalue _alpha) false false))
      (:`Finished`
        (set `self.CanMove` false)
        (`KismetSystemLibrary.Delay` 3.0)
        (set `self.MoveBack` true)
        (bind (_direction_2 _alpha_2) (`Timeline|Close door` :!via `SetNewTime` :!label _label_2)
          (:`Update`
            (`self.K2_SetActorRelativeLocation` _doortoopen (`KismetMathLibrary.VLerp` _returnvalue _location _alpha_2) false false))
          (:`Finished`
            (set `self.MoveBack` false)
            (goto _label :!via `SetNewTime`)))))
    (elif (`self.MoveBack`)
      (goto _label_2))))

(fn `UserConstructionScript`)