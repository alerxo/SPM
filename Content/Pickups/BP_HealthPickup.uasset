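; BP_HealthPickup is a health pickup that bobs its cube up and down in an endless eased MoveComponentTo loop started on BeginPlay.
; When the player pawn overlaps it below full health, it restores health through the pawn's HealthComponent.
; It then passes itself to the game mode's SavePickupMessage, destroys itself, shows a pickup widget and plays a 2D sound.
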(event `self.ReceiveBeginPlay`
  (bind _cube (`self.Cube`))
  (if (not (`self.Moving?`)) :!label _label
    (set `self.Moving?` true)
    (`KismetSystemLibrary.MoveComponentTo` _cube (0.0 0.0 15.0) (struct) true true 1.0)
    (`KismetSystemLibrary.MoveComponentTo` _cube (0.0 0.0 -15.0) (struct) true true 1.0)
    (set `self.Moving?` false)
    (goto _label)))

(event `self.ReceiveActorBeginOverlap`
  (params (OtherActor :type "Actor Object Reference"))
  (bind _returnvalue (`GameplayStatics.GetPlayerPawn` 0))
  (bind _returnvalue_2 (`self.GetComponentByClass` _returnvalue "/Script/SPM.HealthComponent"))
  (if (and (< (`HealthComponent.GetHealthPercentage` _returnvalue_2) 1.0) (== OtherActor _returnvalue))
    (bind _returnvalue_3 (`self.GetHealthToRestore`))
    (`HealthComponent.RestoreHealth` _returnvalue_2 _returnvalue_3)
    (message `/Game/SaveSystem/BPI_SaveObjects.SavePickup` (`GameplayStatics.GetGameMode`) self)
    (`self.K2_DestroyActor`)
    (bind _returnvalue_4 (`|CreateWidget` "/Game/UI/UI_Health_Pickup.UI_Health_Pickup_C" (`GameplayStatics.GetPlayerController` 0)))
    (`UserWidget.AddToViewport` _returnvalue_4 0)
    (`GameplayStatics.PlaySound2D` "/Game/Audio/SFX/UI/SFX_UI_Health_Pickup.SFX_UI_Health_Pickup" 1.0 1.0 0.0 null null)))

(fn `UserConstructionScript`)