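; Health pickup, likely dropped by enemies, that restores player health and despawns after a timer.
; Tick counts down TimeToDespawn and destroys the actor when it runs out.
; On overlap with player pawn 0 while below full health, it passes GetHealthToRestore to the pawn's HealthComponent.
; It then destroys itself, shows the UI_Health_Pickup widget and plays a 2D pickup sound.
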(event `self.ReceiveTick`
  (params (DeltaSeconds :type "Float (single-precision)"))
  (bind _returnvalue (- (`self.TimeToDespawn`) DeltaSeconds))
  ;[1 1 1] Auto Destroys after a timer
  (set `self.TimeToDespawn` _returnvalue)
  (if (<= _returnvalue 0.0)
    (`self.K2_DestroyActor`)))

(event `self.ReceiveActorBeginOverlap`
  (params (OtherActor :type "Actor Object Reference"))
  (bind _returnvalue (`GameplayStatics.GetPlayerPawn` 0))
  (bind _returnvalue_2 (`self.GetComponentByClass` _returnvalue "/Script/SPM.HealthComponent"))
  (if (and (< (`HealthComponent.GetHealthPercentage` _returnvalue_2) 1.0) (== OtherActor _returnvalue))
    (bind _returnvalue_3 (`self.GetHealthToRestore`))
    (`HealthComponent.RestoreHealth` _returnvalue_2 _returnvalue_3)
    (`self.K2_DestroyActor`)
    (bind _returnvalue_4 (`|CreateWidget` "/Game/UI/UI_Health_Pickup.UI_Health_Pickup_C" (`GameplayStatics.GetPlayerController` 0)))
    (`UserWidget.AddToViewport` _returnvalue_4 0)
    (`GameplayStatics.PlaySound2D` "/Game/Audio/SFX/UI/SFX_UI_Health_Pickup.SFX_UI_Health_Pickup" 1.0 1.0 0.0 null null)))

(fn `UserConstructionScript`)