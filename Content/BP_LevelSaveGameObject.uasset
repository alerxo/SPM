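; BP_LevelSaveGameObject holds per-level saved progress for collected pickups and killed enemies, and applies it by removing those actors.
; LoadCollectedPickups loops over CurrentPickups and LoadKilledEnemies loops over KilledEnemies, destroying each entry that is still valid.
; Both work directly on stored actor references, and the file contains no logic that fills the arrays or saves them.
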(fn `LoadCollectedPickups`
  (bind _currentpickups (`self.CurrentPickups`))
  (if (> (`KismetArrayLibrary.Array_Length` _currentpickups) 0)
    (for _array_element _currentpickups
      (`/Engine/EditorBlueprintResources/StandardMacros.IsValid` _array_element
        (:`Is Valid`
          (`Actor.K2_DestroyActor` _array_element))))))

(fn `LoadKilledEnemies`
  (bind _killedenemies (`self.KilledEnemies`))
  (if (> (`KismetArrayLibrary.Array_Length` _killedenemies) 0)
    (for _array_element _killedenemies
      (`/Engine/EditorBlueprintResources/StandardMacros.IsValid` _array_element
        (:`Is Valid`
          (`Actor.K2_DestroyActor` _array_element))))))