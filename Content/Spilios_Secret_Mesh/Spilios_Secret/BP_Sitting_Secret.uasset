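; BP_Sitting_Secret is a secret collectible pickup built around a DavidJrSitting component that bobs up and down.
; BeginPlay runs an endless eased MoveComponentTo loop between two relative heights, guarded by a Moving flag.
; When the player character overlaps Pickup_Collider, it increments the first-person character's Collectibles count and has the game mode save secret and pickup messages.
; It then destroys itself and plays a pickup sound.
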(event `self.ReceiveBeginPlay`
  (bind _davidjrsitting (`self.DavidJrSitting`))
  (`|ExecutionSequence`
    (:`then_0`
      (if (not (`self.Moving?`)) :!label _label
        (set `self.Moving?` true)
        (`KismetSystemLibrary.MoveComponentTo` _davidjrsitting (0.0 0.0 15.0) (struct) true true 1.5)
        (`KismetSystemLibrary.MoveComponentTo` _davidjrsitting (0.0 0.0 -15.0) (struct) true true 1.5)
        (set `self.Moving?` false)
        (goto _label)))))

(event `self.Pickup_Collider.OnComponentBeginOverlap`
  (params (OverlappedComponent :type "PrimitiveComponent Object Reference") (OtherActor :type "Actor Object Reference") (OtherComp :type "PrimitiveComponent Object Reference") (OtherBodyIndex :type Integer) (bFromSweep :type Boolean) (SweepResult :type "HitResult Structure (by ref)"))
  (bind _returnvalue (`GameplayStatics.GetPlayerCharacter` 0))
  (bind _returnvalue_2 (`GameplayStatics.GetGameMode`))
  (if (== OtherActor _returnvalue)
    ;[1 1 1] Add counter. max should be 3
    (bind _asbp_first_person_character (cast `/Game/FirstPerson/Blueprints/BP_FirstPersonCharacter` _returnvalue))
    (bind _result (`/Engine/EditorBlueprintResources/StandardMacros.IncrementInt` (`/Game/FirstPerson/Blueprints/BP_FirstPersonCharacter.Collectibles` _asbp_first_person_character))
      (:`  `
        (set `/Game/FirstPerson/Blueprints/BP_FirstPersonCharacter.Collectibles` _result _asbp_first_person_character)
        (message `/Game/SaveSystem/BPI_SaveObjects.SaveSecret` _returnvalue_2)
        (message `/Game/SaveSystem/BPI_SaveObjects.SavePickup` _returnvalue_2 self)
        (`self.K2_DestroyActor`)
        (`GameplayStatics.PlaySound2D` "/Game/Audio/SFX/Objectives/Secret/SFX_Secret_Picked.SFX_Secret_Picked" 1.0 1.0 0.0 null null)))))

(fn `UserConstructionScript`)