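; BP_WallbreakerActor is the Wallbreaker melee enemy, exposing attack and AI perception reactions.
; Attack plays an animation directly on the mesh, then restores the walk AnimBlueprint after a fixed delay.
; PlayerSeen and Investigate write the blackboard Behaviour enum, with Investigate also storing a location but only acting when no higher behaviour is set.
; On destruction it spawns a Niagara morph effect at its transform.
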(event `self.ReceiveBeginPlay`)

(event `self.ReceiveTick`
  (params (DeltaSeconds :type "Float (single-precision)")))

(event `Attack`
  (`SkeletalMeshComponent.PlayAnimation` (`self.Mesh`) "/Game/Animations/Melee_Attack/Melee_Enemy_Test_Attack_Anim.Melee_Enemy_Test_Attack_Anim" false)
  (`KismetSystemLibrary.Delay` 2.0)
  (`SkeletalMeshComponent.SetAnimInstanceClass` (`self.Mesh`) "/Game/Animations/Melee_Walk/Melee_Enemy_Test_Walk_Skeleton_AnimBlueprint.Melee_Enemy_Test_Walk_Skeleton_AnimBlueprint_C"))

(event `self.ReceiveDestroyed`
  (`NiagaraFunctionLibrary.SpawnSystemAtLocation` "/Game/Particle/NG_Enemy_Morph_BigDUde.NG_Enemy_Morph_BigDUde" (`self.K2_GetActorLocation` self) (`self.K2_GetActorRotation` self)))

(event `EnemyInterface.Investigate`
  (params (Location :type "Vector Structure"))
  (bind _returnvalue (`AIBlueprintHelperLibrary.GetBlackboard` null))
  (bind _behaviour (`self.Behaviour`))
  (`/Engine/EditorBlueprintResources/StandardMacros.IsValid` _returnvalue
    (:`Is Valid`
      (if (not (> (`BlackboardComponent.GetValueAsEnum` _returnvalue _behaviour) 0))
        (`BlackboardComponent.SetValueAsEnum` _returnvalue _behaviour 2)
        (`BlackboardComponent.SetValueAsVector` _returnvalue (`self.Location`) Location)))))

(event `EnemyInterface.PlayerSeen`
  (bind _returnvalue (`AIBlueprintHelperLibrary.GetBlackboard` null))
  (`/Engine/EditorBlueprintResources/StandardMacros.IsValid` _returnvalue
    (:`Is Valid`
      (`BlackboardComponent.SetValueAsEnum` _returnvalue (`self.Behaviour`) 1))))

(fn `UserConstructionScript`)