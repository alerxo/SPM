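; Fireball projectile actor that handles the impact effects of a fireball attack and breaks nearby Chaos destructibles.
; DestroywithFireball runs once, showing an animated hit-indicator widget, then spawning the burst effect, playing impact sound and emitting noise attributed to the player.
; It then uses Field System physics fields sized by its Sphere component: external strain to fracture clusters, and culled radial velocity to push pieces outward.
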(event `self.DestroyWithFireball`
  (bind _returnvalue (`self.K2_GetActorLocation`))
  (bind _sphere (`self.Sphere`))
  (bind _fieldsystem (`self.FieldSystem`))
  (bind _returnvalue_2 (`SceneComponent.K2_GetComponentLocation` _sphere))
  (bind _returnvalue_3 (`RadialFalloff.SetRadialFalloff` (`self.RadialFalloff`) 5000000.0 0.0 1.0 0.0 (`SphereComponent.GetUnscaledSphereRadius` _sphere) _returnvalue_2 "Field_FallOff_None"))
  (`/Engine/EditorBlueprintResources/StandardMacros.DoOnce` false
    (:`Completed`
      (`|ExecutionSequence`
        (:`then_0`
          (bind _returnvalue_4 (`|CreateWidget` "/Game/UI/WB_HitIndicator.WB_HitIndicator_C"))
          (`UserWidget.AddToViewport` _returnvalue_4 0)
          (`UserWidget.PlayAnimation` _returnvalue_4 (`/Game/UI/WB_HitIndicator.Hit` _returnvalue_4) 0.0 1 "Forward" 1.0 false))
        (:`then_1`
          (`SceneComponent.K2_SetWorldRotation` (`self.FireballEffect`) (`self.K2_GetActorRotation`) false false)
          (`NiagaraFunctionLibrary.SpawnSystemAtLocation` "/Game/Particle/Attacks/Fireball/Special_Attack_Burst.Special_Attack_Burst" _returnvalue (`self.K2_GetActorRotation`) (1.0 1.0 1.0) true true "AutoRelease")
          (`self.MakeNoise` 1.0 (`GameplayStatics.GetPlayerCharacter` 0) _returnvalue)
          (`GameplayStatics.PlaySoundAtLocation` "/Game/Audio/SFX/Weapons/SFX_Weapon_Fireball_Impact.SFX_Weapon_Fireball_Impact" _returnvalue (struct) 0.7 1.0 0.0 "/Game/Audio/SFX/Attenuations/ATT_Fireball_Projectile.ATT_Fireball_Projectile" null null null)
          (`FieldSystemComponent.ApplyPhysicsField` _fieldsystem true "Field_ExternalClusterStrain" null _returnvalue_3)
          (`FieldSystemComponent.ApplyPhysicsField` _fieldsystem true "Field_LinearVelocity" null (`CullingField.SetCullingField` (`self.CullingField`) _returnvalue_3 (`RadialVector.SetRadialVector` (`self.RadialVector`) 1000.0 _returnvalue_2) "Field_Culling_Outside")))))))

(fn `UserConstructionScript`)