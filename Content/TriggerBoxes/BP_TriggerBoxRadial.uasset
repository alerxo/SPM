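; BP_TriggerBoxRadial is a trigger box that calls RemoveRadial when the player character enters it.
; Begin overlap opens a Gate and then immediately enters it through a Sequence, firing the call once per entry, and end overlap closes the Gate.
; Disconnected leftovers include a retriggerable delay, an IA_Dash key query and an EnableInput call, none of which run.
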(event `self.ReceiveActorBeginOverlap`
  (params (OtherActor :type "Actor Object Reference"))
  (if (== OtherActor (`GameplayStatics.GetPlayerCharacter` 0))
    (`|ExecutionSequence`
      (:`then_0`
        (goto _label :!via `Open`))
      (:`then_1`
        (`/Engine/EditorBlueprintResources/StandardMacros.Gate` true :!label _label
          (:`Exit`
            (`self.RemoveRadial`)))))))

(event `self.ReceiveActorEndOverlap`
  (params (OtherActor :type "Actor Object Reference"))
  (if (== (`GameplayStatics.GetPlayerCharacter` 0) OtherActor)
    (goto _label :!via `Close`)))

(fn `UserConstructionScript`)